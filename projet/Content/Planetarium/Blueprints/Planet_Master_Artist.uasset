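; Artist-configurable master planet Blueprint that builds a planet's look from exposed variables in its construction script.
; It creates dynamic material instances for the surface, cloud, atmosphere and north polar ice meshes, while both polar cloud meshes get a static material.
; Variables feed their parameters: height-banded terrain from ocean to mountains with detail maps, cloud noise and blending, three-band Fresnel atmosphere colour, and ice shading.
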(fn ConstructionScript
  (bind _planet_sphere_clouds_polar_mat (Variables|Atmosphere|GetPlanet_Sphere_Clouds_Polar_Mat))
  (bind _ice_polar_mat (Variables|Planet|GetIce_Polar_Mat))
  (bind _ice_polar_n (Variables|Default|GetIce_Polar_N))
  (bind _planet_sphere_clouds (Variables|Default|GetPlanet_Sphere_Clouds))
  (bind _planet_sphere (Variables|Default|GetPlanet_Sphere))
  (Rendering|Material|SetMaterial _planet_sphere 0 (stale _returnvalue_3))
  (Rendering|Material|SetMaterial _planet_sphere_clouds 0 (stale _returnvalue_2))
  (Rendering|Material|SetMaterial (Variables|Default|GetPlanet_Sphere_Clouds_Polar_N) 0 _planet_sphere_clouds_polar_mat)
  (Rendering|Material|SetMaterial (Variables|Default|GetPlanet_Sphere_Clouds_Polar_S) 0 _planet_sphere_clouds_polar_mat)
  (Rendering|Material|SetMaterial (Variables|Default|GetPlanet_Sphere_Atmosphere) 0 (stale _returnvalue))
  (bind _returnvalue (Rendering|Material|CreateDynamicMaterialInstance (Variables|Default|GetPlanet_Sphere_Atmosphere) 0 (Variables|Atmosphere|GetPlanet_Sphere_Atmosphere_Mat) :!class /Script/Engine.PrimitiveComponent))
  (Rendering|Material|SetScalarParameterValue _returnvalue "Atmo_Alpha_In" (Variables|Atmosphere|GetAtmo_Alpha_In_Var) :!class /Script/Engine.MaterialInstanceDynamic)
  (Rendering|Material|SetScalarParameterValue _returnvalue "Atmo_Alpha_Mid" (Variables|Atmosphere|GetAtmo_Alpha_Mid_Var) :!class /Script/Engine.MaterialInstanceDynamic)
  (Rendering|Material|SetScalarParameterValue _returnvalue "Fresnel_BaseRef" (Variables|Atmosphere|GetFresnel_BaseRef) :!class /Script/Engine.MaterialInstanceDynamic)
  (Rendering|Material|SetScalarParameterValue _returnvalue "Fresnel_Exponet" (Variables|Atmosphere|GetFresnel_Exponet) :!class /Script/Engine.MaterialInstanceDynamic)
  (Rendering|Material|SetScalarParameterValue _returnvalue "Atmo_Alpha_Out" (Variables|Atmosphere|GetAtmo_Alpha_Out_Var) :!class /Script/Engine.MaterialInstanceDynamic)
  (Rendering|Material|SetVectorParameterValue _returnvalue "Amorpher_color_In" (Variables|Atmosphere|GetAtmo_color_In_Var) :!class /Script/Engine.MaterialInstanceDynamic)
  (Rendering|Material|SetVectorParameterValue _returnvalue "Amorpher_color_Mid" (Variables|Atmosphere|GetAtmo_color_Mid_Var) :!class /Script/Engine.MaterialInstanceDynamic)
  (Rendering|Material|SetVectorParameterValue _returnvalue "Amorpher_color_Out" (Variables|Atmosphere|GetAtmo_color_Out_Var) :!class /Script/Engine.MaterialInstanceDynamic)
  (bind _returnvalue_2 (Rendering|Material|CreateDynamicMaterialInstance _planet_sphere_clouds 0 (Variables|Atmosphere|GetPlanet_Sphere_Clouds_Mat) :!class /Script/Engine.PrimitiveComponent))
  (Rendering|Material|SetTextureParameterValue _returnvalue_2 "World_Hight_and_Compnents" (Variables|Atmosphere|GetWorld_Hight_and_Compnents_Var))
  (Rendering|Material|SetScalarParameterValue _returnvalue_2 "Land_Clouds_Blend" (Variables|Atmosphere|GetLand_Clouds_Blend_Var) :!class /Script/Engine.MaterialInstanceDynamic)
  (Rendering|Material|SetScalarParameterValue _returnvalue_2 "Clouds_A_Clamp_Max" (Variables|Atmosphere|GetClouds_A_Clamp_Max) :!class /Script/Engine.MaterialInstanceDynamic)
  (Rendering|Material|SetVectorParameterValue _returnvalue_2 "Clouds_Colour_ADD" (Variables|Atmosphere|GetClouds_Colour_ADD_Var) :!class /Script/Engine.MaterialInstanceDynamic)
  (Rendering|Material|SetTextureParameterValue _returnvalue_2 "Main_Alpha_Nois_One" (Variables|Atmosphere|GetMain_Alpha_Nois_One))
  (Rendering|Material|SetTextureParameterValue _returnvalue_2 "World_HigMain_Alpha_Cloudes_Oneht_and_Compnents" (Variables|Atmosphere|GetMain_Alpha_Cloudes_One))
  (Rendering|Material|SetTextureParameterValue _returnvalue_2 "Main_Alpha_Nois_Two" (Variables|Atmosphere|GetMain_Alpha_Nois_Two))
  (Rendering|Material|SetTextureParameterValue _returnvalue_2 "Main_Alpha_Cloudes_Two" (Variables|Atmosphere|GetMain_Alpha_Cloudes_Two))
  (Rendering|Material|SetVectorParameterValue _returnvalue_2 "Clouds_Opacity_Mul" (Variables|Atmosphere|GetClouds_Opacity_Mul_Var) :!class /Script/Engine.MaterialInstanceDynamic)
  (bind _returnvalue_3 (Rendering|Material|CreateDynamicMaterialInstance _planet_sphere 0 (Variables|Planet|GetPlanet_Sphere_Mat) :!class /Script/Engine.PrimitiveComponent))
  (Rendering|Material|SetTextureParameterValue _returnvalue_3 "World_Hight_and_Compnents_Planet" (Variables|Planet|GetWorld_Hight_and_Compnents_Planet_Var))
  (Rendering|Material|SetScalarParameterValue _returnvalue_3 "Ocean_Hight" (Variables|Planet|GetOcean_Hight_Var) :!class /Script/Engine.MaterialInstanceDynamic)
  (Rendering|Material|SetScalarParameterValue _returnvalue_3 "Ocean_Hight_Borders" (Variables|Planet|GetOcean_Hight_Borders_Var) :!class /Script/Engine.MaterialInstanceDynamic)
  (Rendering|Material|SetScalarParameterValue _returnvalue_3 "Ocean_Hight_Borders_Power" (Variables|Planet|GetOcean_Hight_Borders_Power) :!class /Script/Engine.MaterialInstanceDynamic)
  (Rendering|Material|SetScalarParameterValue _returnvalue_3 "Costline_Hight" (Variables|Planet|GetCostline_Hight) :!class /Script/Engine.MaterialInstanceDynamic)
  (Rendering|Material|SetScalarParameterValue _returnvalue_3 "Ocean_Hight_Borders_Power" (Variables|Planet|GetCostline_Hight_Borders) :!class /Script/Engine.MaterialInstanceDynamic)
  (Rendering|Material|SetScalarParameterValue _returnvalue_3 "Ocean_Hight_Borders_Power" (Variables|Planet|GetCostline_Hight_Borders_Power) :!class /Script/Engine.MaterialInstanceDynamic)
  (Rendering|Material|SetScalarParameterValue _returnvalue_3 "Land_Hight" (Variables|Planet|GetLand_Hight) :!class /Script/Engine.MaterialInstanceDynamic)
  (Rendering|Material|SetScalarParameterValue _returnvalue_3 "Land_Hight_Border" (Variables|Planet|GetLand_Hight_Border) :!class /Script/Engine.MaterialInstanceDynamic)
  (Rendering|Material|SetScalarParameterValue _returnvalue_3 "Land_Hight_Border_Power" (Variables|Planet|GetLand_Hight_Border_Power) :!class /Script/Engine.MaterialInstanceDynamic)
  (Rendering|Material|SetScalarParameterValue _returnvalue_3 "Flat_Land_Hight" (Variables|Planet|GetFlat_Land_Hight) :!class /Script/Engine.MaterialInstanceDynamic)
  (Rendering|Material|SetScalarParameterValue _returnvalue_3 "Flat_Land_Hight_Border" (Variables|Planet|GetFlat_Land_Hight_Border) :!class /Script/Engine.MaterialInstanceDynamic)
  (Rendering|Material|SetScalarParameterValue _returnvalue_3 "Flat_Land_Hight_Border_Power" (Variables|Planet|GetFlat_Land_Hight_Border_Power) :!class /Script/Engine.MaterialInstanceDynamic)
  (Rendering|Material|SetScalarParameterValue _returnvalue_3 "Forests_Hight" (Variables|Planet|GetForests_Hight) :!class /Script/Engine.MaterialInstanceDynamic)
  (Rendering|Material|SetScalarParameterValue _returnvalue_3 "Forests_Hight_Border" (Variables|Planet|GetForests_Hight_Border) :!class /Script/Engine.MaterialInstanceDynamic)
  (Rendering|Material|SetScalarParameterValue _returnvalue_3 "Forests_Hight_Border_Power" (Variables|Planet|GetForests_Hight_Border_Power) :!class /Script/Engine.MaterialInstanceDynamic)
  (Rendering|Material|SetScalarParameterValue _returnvalue_3 "Hills_Hight" (Variables|Planet|GetHills_Hight) :!class /Script/Engine.MaterialInstanceDynamic)
  (Rendering|Material|SetScalarParameterValue _returnvalue_3 "Hills_Hight_Border" (Variables|Planet|GetMountains_Hight_Border) :!class /Script/Engine.MaterialInstanceDynamic)
  (Rendering|Material|SetScalarParameterValue _returnvalue_3 "Hills_Hight_Border_Power" (Variables|Planet|GetHills_Hight_Border_Power) :!class /Script/Engine.MaterialInstanceDynamic)
  (Rendering|Material|SetScalarParameterValue _returnvalue_3 "Mountains_Hight" (Variables|Planet|GetMountains_Hight) :!class /Script/Engine.MaterialInstanceDynamic)
  (Rendering|Material|SetScalarParameterValue _returnvalue_3 "Mountains_Hight_Border" (Variables|Planet|GetMountains_Hight_Border) :!class /Script/Engine.MaterialInstanceDynamic)
  (Rendering|Material|SetTextureParameterValue _returnvalue_3 "Coastline_Texture_cc" (Variables|Planet|GetCoastline_Texture_cc))
  (Rendering|Material|SetTextureParameterValue _returnvalue_3 "Flat_Land_Texture_cc" (Variables|Planet|GetFlat_Land_Texture_cc))
  (Rendering|Material|SetTextureParameterValue _returnvalue_3 "Forests_Texture_cc" (Variables|Planet|GetForests_Texture_cc))
  (Rendering|Material|SetTextureParameterValue _returnvalue_3 "Hills_Texture_cc" (Variables|Planet|GetHills_Texture_cc))
  (Rendering|Material|SetTextureParameterValue _returnvalue_3 "Mountains_Texture_cc" (Variables|Planet|GetMountains_Texture_cc))
  (Rendering|Material|SetTextureParameterValue _returnvalue_3 "Flat_Land_Texture_nm" (Variables|Planet|GetFlat_Land_Texture_nm))
  (Rendering|Material|SetTextureParameterValue _returnvalue_3 "Forests_Texture_nm" (Variables|Planet|GetForests_Texture_nm))
  (Rendering|Material|SetTextureParameterValue _returnvalue_3 "Hills_Texture_nm" (Variables|Planet|GetHills_Texture_nm))
  (Rendering|Material|SetTextureParameterValue _returnvalue_3 "DetailTextur_nm" (Variables|Planet|GetDetailTextur_nm))
  (Rendering|Material|SetTextureParameterValue _returnvalue_3 "DetailTextur_cc" (Variables|Planet|GetDetailTextur_cc))
  (Rendering|Material|SetVectorParameterValue _returnvalue_3 "Diffus_Master_Multiply" (Variables|Planet|GetDiffus_Master_Multiply) :!class /Script/Engine.MaterialInstanceDynamic)
  (Rendering|Material|SetScalarParameterValue _returnvalue_3 "Metallic_Add" (Variables|Planet|GetMetallic_Add) :!class /Script/Engine.MaterialInstanceDynamic)
  (Rendering|Material|SetScalarParameterValue _returnvalue_3 "Metallic_Multiply" (Variables|Planet|GetMetallic_Multiply) :!class /Script/Engine.MaterialInstanceDynamic)
  (Rendering|Material|SetScalarParameterValue _returnvalue_3 "Specular_Multiply" (Variables|Planet|GetSpecular_Multiply) :!class /Script/Engine.MaterialInstanceDynamic)
  (Rendering|Material|SetScalarParameterValue _returnvalue_3 "Roughness_Power" (Variables|Planet|GetRoughness_Power) :!class /Script/Engine.MaterialInstanceDynamic)
  (Rendering|Material|SetScalarParameterValue _returnvalue_3 "Detail_Scale" (Variables|Planet|GetDetail_Scale) :!class /Script/Engine.MaterialInstanceDynamic)
  (Rendering|Material|SetScalarParameterValue _returnvalue_3 "Detail_Diffuse_Blend" (Variables|Planet|GetDetail_Diffuse_Blend) :!class /Script/Engine.MaterialInstanceDynamic)
  (Rendering|Material|SetScalarParameterValue _returnvalue_3 "Detail_Scale" (Variables|Planet|GetDetail_Normal_Blend) :!class /Script/Engine.MaterialInstanceDynamic)
  (Rendering|Material|SetScalarParameterValue _returnvalue_3 "Bump_Offset_Factor" (Variables|Planet|GetBump_Offset_Factor) :!class /Script/Engine.MaterialInstanceDynamic)
  (Rendering|Material|SetMaterial _ice_polar_n 0 _ice_polar_mat)
  (bind _returnvalue_4 (Rendering|Material|CreateDynamicMaterialInstance _ice_polar_n 0 _ice_polar_mat :!class /Script/Engine.PrimitiveComponent))
  (Rendering|Material|SetScalarParameterValue _returnvalue_4 "Ice_Metallic" (Variables|Planet|GetIce_Metallic) :!class /Script/Engine.MaterialInstanceDynamic)
  (Rendering|Material|SetScalarParameterValue _returnvalue_4 "Ice_Specular" (Variables|Planet|GetIce_Specular) :!class /Script/Engine.MaterialInstanceDynamic)
  (Rendering|Material|SetScalarParameterValue _returnvalue_4 "Ice_Roughnes" (Variables|Planet|GetIce_Roughnes) :!class /Script/Engine.MaterialInstanceDynamic)
  (Rendering|Material|SetScalarParameterValue _returnvalue_4 "Ice_Border_Extend" (Variables|Planet|GetIce_Border_Extend) :!class /Script/Engine.MaterialInstanceDynamic)
  (Rendering|Material|SetVectorParameterValue _returnvalue_4 "Ice_Diffuse_Multiplay" (Variables|Planet|GetIce_Diffuse_Multiplay) :!class /Script/Engine.MaterialInstanceDynamic)
  (Rendering|Material|SetTextureParameterValue _returnvalue_4 "Ice_Polar_Alpha_Detail" (Variables|Planet|GetIce_Polar_Alpha_Detail))
  (Rendering|Material|SetTextureParameterValue _returnvalue_4 "Ice_Polar_Alpha_A" (Variables|Planet|GetIce_Polar_Alpha_A))
  (Rendering|Material|SetTextureParameterValue _returnvalue_4 "Ice_Polar_Alpha_B" (Variables|Planet|GetIce_Polar_Alpha_B))
  (Rendering|Material|SetTextureParameterValue _returnvalue_4 "Ice_Polar_Normal" (Variables|Planet|GetIce_Polar_Normal))
  (Rendering|Material|SetTextureParameterValue _returnvalue_4 "Flat_Land_Texture_nm" (Variables|Planet|GetIce_Polar_Normal_detail)))