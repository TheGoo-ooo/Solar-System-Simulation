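; Planetarium universe backdrop that builds a star sphere, polar caps, sun light with disk, and galaxy region overlay in its construction script.
; It publishes the light's position and direction as vector parameters and feeds sun and Milky Way settings into dynamic material instances.
; Scale indices swap preset addon meshes for sun and region.
; Visible regions use a stars-only sphere material, while index 9 hides the region and applies the full Milky Way material.
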(fn ConstructionScript
  (bind _returnvalue (Transformation|GetActorTransform))
  (bind _universe_sphere (Variables|Default|GetUniverse_Sphere))
  (bind _universe_sphere_material (Variables|Default|GetUniverse_Sphere_Material))
  (bind _universe_sphere_2 (Variables|Default|GetUniverse_Sphere))
  (bind _universe_sphere_polar (Variables|Default|GetUniverse_Sphere_Polar))
  (bind _sun (Variables|Default|GetSun))
  (bind _universe_region (Variables|Default|GetUniverse_Region))
  (bind _the_sun_01 (Variables|Default|GetThe_Sun_01))
  (bind _the_sun_01_mat (Variables|Default|GetThe_sun_01_Mat))
  (bind _output_get (Variables|Default|SetSun_Rotation (Variables|Default|GetSun_Rotation)))
  (Transformation|SetWorldRotation (Variables|Default|GetSun) _output_get false false)
  (Utilities|FlowControl|Sequence
    (:then_0
      ;[1 1 1] Get Position and Direction of Sun's Light
      (Rendering|Material|SetVectorParameterValue 0 "LightPosition" (Math|Conversions|ToLinearColor(Vector) (Math|Vector|RotateVector (* (.scale _returnvalue) "-50000.000000, 0, 0") (.rotation _returnvalue))) :!class /Script/Engine.KismetMaterialLibrary)
      (Rendering|Material|SetVectorParameterValue 0 "LightVector" (Math|Conversions|ToLinearColor(Vector) (Math|Vector|GetForwardVector (Variables|Default|GetSun))) :!class /Script/Engine.KismetMaterialLibrary))
    (:then_1
      (Transformation|SetRelativeRotation (Variables|Default|GetUniverse_Region) (Variables|Default|GetRegion_Rotation) false false)
      (Rendering|Components|Light|SetLightColor _sun (Variables|Default|GetSun_Light_color) true)
      (Rendering|Components|Light|SetIntensity _sun (Variables|Default|GetSun_Light_Power))
      (Rendering|Material|SetMaterial _universe_sphere_2 0 _universe_sphere_material)
      (Rendering|Material|SetMaterial (Variables|Default|GetUniverse_Sphere_Polar_N) 0 _universe_sphere_polar)
      (Rendering|Material|SetMaterial (Variables|Default|GetUniverse_Sphere_Polar_S) 0 _universe_sphere_polar)
      (Rendering|Material|SetMaterial _the_sun_01 0 _the_sun_01_mat)
      (Transformation|AddRelativeRotation _the_sun_01 (Variables|Default|GetSun_Rotation) false false)
      (bind _returnvalue_2 (Rendering|Material|CreateDynamicMaterialInstance _the_sun_01 0 _the_sun_01_mat :!class /Script/Engine.PrimitiveComponent))
      (Rendering|Material|SetScalarParameterValue _returnvalue_2 "Sun_Brightness_x2" (Variables|Default|GetSun_Brightness_x2) :!class /Script/Engine.MaterialInstanceDynamic)
      (Rendering|Material|SetScalarParameterValue _returnvalue_2 "Sun_Brightness_/2" (Variables|Default|GetSun_Brightness_/2) :!class /Script/Engine.MaterialInstanceDynamic)
      (Rendering|Material|SetScalarParameterValue _returnvalue_2 "Sun_Alpha_boost" (Variables|Default|GetSun_Alpha_boost) :!class /Script/Engine.MaterialInstanceDynamic)
      (Rendering|Material|SetVectorParameterValue _returnvalue_2 "Sun_color" (Variables|Default|GetSun_color) :!class /Script/Engine.MaterialInstanceDynamic)
      (bind _returnvalue_3 (Rendering|Material|CreateDynamicMaterialInstance _universe_sphere_2 0 _universe_sphere_material :!class /Script/Engine.PrimitiveComponent))
      (LocalVariables|SetUniverseSphereMaterialInstance _returnvalue_3)
      (CallFunction|SetDynamicMaterialInstanceParameters (Variables|Default|GetMilkyway_Brightness) (Variables|Default|GetMilkyWay_Stars) (Variables|Default|GetMilkyWay_Stars_Power) (Variables|Default|GetMilkyWay_Outer_Stars) (Variables|Default|GetRegion%20Texture) (LocalVariables|GetUniverseSphereMaterialInstance))
      (Rendering|Material|SetMaterial (Variables|Default|GetUniverse_Region) 0 (Variables|Default|GetRegion%20Galaxy))
      (Utilities|FlowControl|Sequence
        (:then_0
          ;[1 1 1] Set Sun Disk
          (switch int (Variables|Default|GetSun_Scale)
            (:Default
              (Components|StaticMesh|SetStaticMesh _the_sun_01 "/Game/Planetarium/Meshes/Universe_Sphere_Addon_01.Universe_Sphere_Addon_01" :!label _label))
            (:0
              (Components|StaticMesh|SetStaticMesh _the_sun_01 0))
            (:1
              (goto _label))
            (:2
              (Components|StaticMesh|SetStaticMesh _the_sun_01 "/Game/Planetarium/Meshes/Universe_Sphere_Addon_02.Universe_Sphere_Addon_02"))
            (:3
              (Components|StaticMesh|SetStaticMesh _the_sun_01 "/Game/Planetarium/Meshes/Universe_Sphere_Addon_03.Universe_Sphere_Addon_03"))
            (:4
              (Components|StaticMesh|SetStaticMesh _the_sun_01 "/Game/Planetarium/Meshes/Universe_Sphere_Addon_04.Universe_Sphere_Addon_04"))
            (:5
              (Components|StaticMesh|SetStaticMesh _the_sun_01 "/Game/Planetarium/Meshes/Universe_Sphere_Addon_05.Universe_Sphere_Addon_05"))
            (:6
              (Components|StaticMesh|SetStaticMesh _the_sun_01 "/Game/Planetarium/Meshes/Universe_Sphere_Addon_06.Universe_Sphere_Addon_06"))
            (:7
              (Components|StaticMesh|SetStaticMesh _the_sun_01 "/Game/Planetarium/Meshes/Universe_Sphere_Addon_07.Universe_Sphere_Addon_07"))
            (:8
              (Components|StaticMesh|SetStaticMesh _the_sun_01 "/Game/Planetarium/Meshes/Universe_Sphere_Addon_08.Universe_Sphere_Addon_08"))))
        (:then_1
          (switch int (Variables|Default|GetUniverse_Region_Scale)
            (:Default
              (Components|StaticMesh|SetStaticMesh _universe_region "/Game/Planetarium/Meshes/Universe_Sphere_Addon_07.Universe_Sphere_Addon_07" :!label _label_2)
              (Rendering|Material|SetMaterial (Variables|Default|GetUniverse_Sphere) 0 (Variables|Default|GetUniverse_Sphere_Stars_Only_Material) :!label _label_3))
            (:0
              (Components|StaticMesh|SetStaticMesh _universe_region 0 :!label _label_4))
            (:1
              (Components|StaticMesh|SetStaticMesh _universe_region "/Game/Planetarium/Meshes/Universe_Sphere_Addon_01.Universe_Sphere_Addon_01")
              (goto _label_3))
            (:2
              (Components|StaticMesh|SetStaticMesh _universe_region "/Game/Planetarium/Meshes/Universe_Sphere_Addon_02.Universe_Sphere_Addon_02")
              (goto _label_3))
            (:3
              (Components|StaticMesh|SetStaticMesh _universe_region "/Game/Planetarium/Meshes/Universe_Sphere_Addon_03.Universe_Sphere_Addon_03")
              (goto _label_3))
            (:4
              (Components|StaticMesh|SetStaticMesh _universe_region "/Game/Planetarium/Meshes/Universe_Sphere_Addon_04.Universe_Sphere_Addon_04")
              (goto _label_3))
            (:5
              (Components|StaticMesh|SetStaticMesh _universe_region "/Game/Planetarium/Meshes/Universe_Sphere_Addon_05.Universe_Sphere_Addon_05")
              (goto _label_3))
            (:6
              (Components|StaticMesh|SetStaticMesh _universe_region "/Game/Planetarium/Meshes/Universe_Sphere_Addon_06.Universe_Sphere_Addon_06")
              (goto _label_3))
            (:7
              (goto _label_2))
            (:8
              (Components|StaticMesh|SetStaticMesh _universe_region "/Game/Planetarium/Meshes/Universe_Sphere_Addon_08.Universe_Sphere_Addon_08")
              (goto _label_3))
            (:9
              (Utilities|FlowControl|Sequence
                (:then_0
                  (Rendering|Material|SetMaterial _universe_sphere 0 (LocalVariables|GetUniverseSphereMaterialInstance))
                  (bind _returnvalue_4 (Rendering|Material|CreateDynamicMaterialInstance _universe_sphere 0 (LocalVariables|GetUniverseSphereMaterialInstance) :!class /Script/Engine.PrimitiveComponent))
                  (CallFunction|SetDynamicMaterialInstanceParameters (Variables|Default|GetMilkyway_Brightness) (Variables|Default|GetMilkyWay_Stars) (Variables|Default|GetMilkyWay_Stars_Power) (Variables|Default|GetMilkyWay_Outer_Stars) (Variables|Default|GetRegion%20Texture) _returnvalue_4))
                (:then_1
                  (goto _label_4))))))))))

(fn SetDynamicMaterialInstanceParameters
  (params (Milkyway_Brightness :type Float%20%28single-precision%29) (MilkyWay_Stars :type Float%20%28single-precision%29) (MilkyWay_Stars_Power :type Float%20%28single-precision%29) (MilkyWay_Outer_Stars :type Float%20%28single-precision%29) (Region%20Texture :type Texture%20Object%20Reference) (Dynamic%20Material%20Instance :type Material%20Instance%20Dynamic%20Object%20Reference))
  (Rendering|Material|SetScalarParameterValue Dynamic%20Material%20Instance "Milkyway_Brightness" Milkyway_Brightness :!class /Script/Engine.MaterialInstanceDynamic)
  (Rendering|Material|SetScalarParameterValue Dynamic%20Material%20Instance "MilkyWay_Stars" MilkyWay_Stars :!class /Script/Engine.MaterialInstanceDynamic)
  (Rendering|Material|SetScalarParameterValue Dynamic%20Material%20Instance "MilkyWay_Stars_Power" MilkyWay_Stars_Power :!class /Script/Engine.MaterialInstanceDynamic)
  (Rendering|Material|SetScalarParameterValue Dynamic%20Material%20Instance "MilkyWay_Outer_Stars" MilkyWay_Outer_Stars :!class /Script/Engine.MaterialInstanceDynamic)
  (Rendering|Material|SetTextureParameterValue Dynamic%20Material%20Instance "MilkyWayTexture" Region%20Texture)
  (return))